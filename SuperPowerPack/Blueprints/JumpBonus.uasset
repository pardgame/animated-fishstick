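; JumpBonus is a spinning pickup that temporarily raises the player character's jump Z velocity.
; It caches that velocity at BeginPlay, and when the player pawn overlaps its box it sets the velocity to the cached value plus ImpactValue.
; It then destroys its box, cube and text components, waits EffectDuration, restores the velocity from the cached value and destroys itself.
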(event `self.ReceiveBeginPlay`
  (set `self.Jump Z Velocity` (`CharacterMovementComponent.JumpZVelocity` (`Character.CharacterMovement` (`GameplayStatics.GetPlayerCharacter` 0)))))

(event `self.ReceiveTick`
  (params (DeltaSeconds :type "Float (single-precision)"))
  (`SceneComponent.K2_AddLocalRotation` (`self.Cube`) (struct :`Pitch` 2.0 :`Yaw` 2.0 :`Roll` 2.0) false false))

(event `self.BoxCollision.OnComponentBeginOverlap`
  (params (OverlappedComponent :type "PrimitiveComponent Object Reference") (OtherActor :type "Actor Object Reference") (OtherComp :type "PrimitiveComponent Object Reference") (OtherBodyIndex :type Integer) (bFromSweep :type Boolean) (SweepResult :type "HitResult Structure (by ref)"))
  (bind _charactermovement (`Character.CharacterMovement` (`GameplayStatics.GetPlayerCharacter` 0)))
  (if (== OtherActor (`GameplayStatics.GetPlayerPawn` 0))
    (bind _output_get (set `CharacterMovementComponent.JumpZVelocity` (+ (`self.impact value`) (`self.Jump Z Velocity`)) _charactermovement))
    (set `self.Jump Z Velocity` _output_get)
    (`ActorComponent.K2_DestroyComponent` (`self.BoxCollision`))
    (`ActorComponent.K2_DestroyComponent` (`self.Cube`))
    (`ActorComponent.K2_DestroyComponent` (`self.TextRender`))
    (`KismetSystemLibrary.Delay` (`self.effect duration`))
    (set `CharacterMovementComponent.JumpZVelocity` (- (`self.Jump Z Velocity`) (`self.impact value`)) _charactermovement)
    (`self.K2_DestroyActor` self)))

(fn `UserConstructionScript`)