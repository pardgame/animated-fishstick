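; SpeedBonus is a pickup actor with a spinning cube and text that temporarily changes the player's walk speed.
; When the player pawn overlaps its box, it adds ImpactValue to MaxWalkSpeed, caches the result and destroys its components.
; After EffectDuration it sets the speed to the cached value minus ImpactValue, overriding any later speed changes, then destroys itself.
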(event `self.ReceiveBeginPlay`
  (set `self.Max Walk Speed` (`CharacterMovementComponent.MaxWalkSpeed` (`Character.CharacterMovement` (`GameplayStatics.GetPlayerCharacter` 0)))))

(event `self.ReceiveTick`
  (params (DeltaSeconds :type "Float (single-precision)"))
  (`SceneComponent.K2_AddLocalRotation` (`self.Cube`) (struct :`Pitch` 2.0 :`Yaw` 2.0 :`Roll` 2.0) false false))

(event `self.BoxCollision.OnComponentBeginOverlap`
  (params (OverlappedComponent :type "PrimitiveComponent Object Reference") (OtherActor :type "Actor Object Reference") (OtherComp :type "PrimitiveComponent Object Reference") (OtherBodyIndex :type Integer) (bFromSweep :type Boolean) (SweepResult :type "HitResult Structure (by ref)"))
  (bind _charactermovement (`Character.CharacterMovement` (`GameplayStatics.GetPlayerCharacter` 0)))
  (if (== OtherActor (`GameplayStatics.GetPlayerPawn` 0))
    (bind _output_get (set `CharacterMovementComponent.MaxWalkSpeed` (+ (`self.impact value`) (`CharacterMovementComponent.MaxWalkSpeed` _charactermovement)) _charactermovement))
    (set `self.Max Walk Speed` _output_get)
    (`ActorComponent.K2_DestroyComponent` (`self.BoxCollision`))
    (`ActorComponent.K2_DestroyComponent` (`self.Cube`))
    (`ActorComponent.K2_DestroyComponent` (`self.TextRender`))
    (`KismetSystemLibrary.Delay` (`self.effect duration`))
    (set `CharacterMovementComponent.MaxWalkSpeed` (- (`self.Max Walk Speed`) (`self.impact value`)) _charactermovement)
    (`self.K2_DestroyActor` self)))

(fn `UserConstructionScript`)